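; Pawn for the kinematic algorithms that pairs its KinematicSeek target with a separate target actor.
; On BeginPlay it spawns a BP_TargetActor at the seek target location and stores the reference.
; UpdateTargetMeshLocation moves that actor's mesh component to the current seek target without sweeping; nothing in this Blueprint calls it, and Tick is unused.
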(event EventBeginPlay
  (bind _returnvalue (Game|SpawnActorfromClass "/Game/Blueprints/BP_TargetActor.BP_TargetActor_C" (Math|Transform|MakeTransform (Variables|/Script/AI_Experiments.KinematicSeekComponent|GetTarget (Variables|Default|GetKinematicSeek))) "Undefined" 0 0))
  (Variables|Default|SetTargetMesh _returnvalue))

(event EventTick
  (params (DeltaSeconds :type Float%20%28single-precision%29)))

(fn ConstructionScript)

(fn UpdateTargetMeshLocation
  (Transformation|SetWorldLocation (Variables|/Game/Blueprints/BP_TargetActor.BP_TargetActor_C|GetTargetMesh (Variables|Default|GetTargetMesh)) (Variables|/Script/AI_Experiments.KinematicSeekComponent|GetTarget (Variables|Default|GetKinematicSeek)) false false))