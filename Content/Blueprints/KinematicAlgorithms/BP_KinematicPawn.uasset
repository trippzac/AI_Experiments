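; BP_KinematicPawn is a pawn that hosts a kinematic movement algorithm and a visual marker for its target.
; On BeginPlay it adds the component given by KinematicMovementClass, so the algorithm is selectable per pawn, and seeds its target from StartingTargetLocation.
; It then spawns a BP_TargetActor at that target, printing an error if the spawn fails.
; UpdateTargetMeshLocation moves the marker's mesh to a new location.
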(event EventBeginPlay
  (bind _returnvalue (Game|AddComponentbyClass (Variables|Default|GetKinematicMovementClass)))
  (bind _output_get (Variables|Default|SetKinematicComponent _returnvalue))
  (bind _output_get_2 (Variables|/Script/AI_Experiments.KinematicMovementComponent|SetTarget _output_get (Variables|Default|GetStartingTargetLocation)))
  (bind _returnvalue_2 (Game|SpawnActorfromClass "/Game/Blueprints/BP_TargetActor.BP_TargetActor_C" (Math|Transform|MakeTransform _output_get_2) "Undefined" 0 0))
  (Utilities|IsValid _returnvalue_2
    (:Is%20Valid
      (Variables|Default|SetTargetMesh _returnvalue_2))
    (:Is%20Not%20Valid
      (Development|PrintString "Mesh not created" true true "(R=0.000000,G=0.660000,B=1.000000,A=1.000000)" 1e+01))))

(fn ConstructionScript)

(fn UpdateTargetMeshLocation
  (params (NewLocation :type Vector))
  (Transformation|SetWorldLocation (Variables|/Game/Blueprints/BP_TargetActor.BP_TargetActor_C|GetTargetMesh (Variables|Default|GetTargetMesh)) NewLocation false false))