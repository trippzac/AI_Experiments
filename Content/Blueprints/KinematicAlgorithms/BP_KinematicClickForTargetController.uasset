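; Player controller that sets a movement target for a kinematic-algorithm pawn by clicking in the world.
; It shows the mouse cursor on BeginPlay, then on left click traces under the cursor on the Visibility channel.
; The hit's X and Y, flattened to the pawn's height, become the KinematicComponent's Target.
; The pawn's target mesh is then moved to that point.
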(event EventBeginPlay
  (Variables|Default|SetbShowMouseCursor true))

(event Input|MouseEvents|LeftMouseButton
  (params (Key :type Key%20Structure :default "None"))
  (bind _returnvalue (Game|Player|GetPlayerPawn 0))
  (bind _returnvalue_2 (Game|GetPlayerController 0))
  (bind (_hitresult _returnvalue_3) (Game|Player|GetHitResultUnderCursorbyChannel _returnvalue_2 "TraceTypeQuery1" true))
  (bind _location (Collision|BreakHitResult _hitresult))
  (bind (_x _y) (Math|Vector|BreakVector _location))
  (:Pressed
    (if _returnvalue_3
      (bind _asbp_kinematic_pawn (Utilities|Casting|CastToBP_KinematicPawn _returnvalue))
      (bind _output_get (Variables|/Script/AI_Experiments.KinematicMovementComponent|SetTarget (Variables|/Game/Blueprints/KinematicAlgorithms/BP_KinematicPawn.BP_KinematicPawn_C|GetKinematicComponent _asbp_kinematic_pawn) (Math|Vector|MakeVector _x _y (.Z (Math|Vector|BreakVector (Transformation|GetActorLocation _returnvalue))))))
      (Default|UpdateTargetMeshLocation _asbp_kinematic_pawn _output_get))))

(fn ConstructionScript)