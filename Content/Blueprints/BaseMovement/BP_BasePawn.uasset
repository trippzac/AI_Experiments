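; BP_BasePawn is a base pawn that seeks toward a target position, shown in the world by a separate target actor.
; BeginPlay adds a seek component, configures BaseMovement with max speed, acceleration and starting target, then spawns BP_TargetActor at that position.
; UpdateTargetMeshLocation keeps both in sync by passing a new position to the movement and moving the target actor's mesh there.
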(event EventBeginPlay
  (bind _startingtargetposition (Variables|Default|GetStartingTargetPosition))
  (Game|AddComponentbyClass "/Script/AI_Experiments.BaseSeekComponent")
  (bind _output_get (Variables|Default|SetBaseMovement 0))
  (Class|BaseMovementComponent|SetMaxSpeed _output_get (Variables|Default|GetMaxSpeed))
  (Class|BaseMovementComponent|SetMaxAcceleration _output_get (Variables|Default|GetMaxAcceleration))
  (Class|BaseMovementComponent|SetTargetPosition _output_get _startingtargetposition)
  (bind _returnvalue (Game|SpawnActorfromClass "/Game/Blueprints/BP_TargetActor.BP_TargetActor_C" (Math|Transform|MakeTransform _startingtargetposition) "Undefined" 0 0))
  (Utilities|IsValid _returnvalue
    (:Is%20Valid
      (Variables|Default|SetTargetActor _returnvalue))
    (:Is%20Not%20Valid
      (Development|PrintString "Mesh not created" true true "(R=0.000000,G=0.660000,B=1.000000,A=1.000000)" 1e+01))))

(fn ConstructionScript)

(fn UpdateTargetMeshLocation
  (params (NewPosition :type Vector))
  (Class|BaseMovementComponent|SetTargetPosition (Variables|Default|GetBaseMovement) NewPosition)
  (Transformation|SetWorldLocation (Variables|/Game/Blueprints/BP_TargetActor.BP_TargetActor_C|GetTargetMesh (Variables|Default|GetTargetActor)) NewPosition false false))